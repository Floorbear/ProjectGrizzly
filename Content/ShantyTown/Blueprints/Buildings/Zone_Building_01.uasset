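; Zone_Building_01 is a building zone actor in ShantyTown that switches a post-process effect for player exposure.
; BeginExposure sets the PostProcess blend weight to full and EndExposure clears it, both only when the passed object is a BP_Player.
; IsLocalPlayer reports whether an object is a locally controlled BP_Player.
; A timeline meant to fade and print the blend weight is left unconnected, so the switch is instant.
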(fn `BeginExposure`
  (params (Object :type "Object Object Reference"))
  (cast `/Game/ProjectGrizzly/Character/BP_Player` Object)
  (set `PostProcessComponent.BlendWeight` 1.0 (`self.PostProcess`)))

(fn `EndExposure`
  (params (Object :type "Object Object Reference"))
  (cast `/Game/ProjectGrizzly/Character/BP_Player` Object)
  (set `PostProcessComponent.BlendWeight` 0.0 (`self.PostProcess`)))

(fn `IsLocalPlayer`
  (params (Object :type "Object Object Reference"))
  (returns (NewParam :type Boolean))
  (bind _asbp_player (cast `/Game/ProjectGrizzly/Character/BP_Player` Object)
    (:`then`
      (return (`Pawn.IsLocallyControlled` _asbp_player)))
    (:`CastFailed`
      (return false))))

(fn `UserConstructionScript`)