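; BP_ItemContainer is an interactable world container holding an inventory that players can open.
; On BeginPlay, the server seeds its Inventory component with a loner patch and an AKM as hardcoded starting items.
; Interact casts the instigator's controller to BP_GrizzlyPC and calls ShowInventory, passing the ItemContainer category and this inventory as the target.
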(event `self.ReceiveBeginPlay`
  (bind _inventory (`self.Inventory`))
  (`/Engine/EditorBlueprintResources/ActorMacros.Switch Has Authority`
    (:`Authority`
      (`InventoryComponent.AddItemToInventory` _inventory "Etc_LonerPatch" 1)
      (`InventoryComponent.AddItemToInventory` _inventory "Weapon_AKM" 1))))

(event `self.Interact`
  (params (_Instigator :type "Actor Object Reference"))
  (bind `_as폰` (cast `Pawn` _Instigator))
  (bind _asbp_grizzly_pc (cast `/Game/ProjectGrizzly/Character/BP_GrizzlyPC` (`Pawn.GetController` `_as폰`)))
  (`GrizzlyPC.ShowInventory` _asbp_grizzly_pc (make `InventoryUI_Parameter` "ItemContainer" (`self.Inventory`))))

(fn `UserConstructionScript`)