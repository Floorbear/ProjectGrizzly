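; BP_ExtractionPoint is an extraction zone where the locally controlled player waits out a countdown to leave the match.
; Entering the Cube shows ExtractionUI and starts a looping countdown timer; leaving clears it and fades the UI, collapsing it after a short delay.
; At zero, a FadeInOut widget plays a fade-out with a bound finish callback.
; A Disconnect function saves the player controller's inventory and runs the disconnect console command.
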(event `self.ReceiveBeginPlay`
  (if (`KismetSystemLibrary.IsValid` (`GameplayStatics.GetPlayerController` 0))
    (if (`Controller.IsLocalController` (`GameplayStatics.GetPlayerController` 0))
      (bind _returnvalue (`|CreateWidget` "/Game/ProjectGrizzly/Map/ExtractionPoint/ExtractionWidget.ExtractionWidget_C" (`GameplayStatics.GetPlayerController` 0) self))
      (bind _output_get (set `self.ExtractionUI` _returnvalue))
      (`UserWidget.AddToViewport` _output_get 0)
      (`Widget.SetVisibility` _output_get "Collapsed"))))

(event `self.Cube.OnComponentBeginOverlap`
  (params (OverlappedComponent :type "PrimitiveComponent Object Reference") (OtherActor :type "Actor Object Reference") (OtherComp :type "PrimitiveComponent Object Reference") (OtherBodyIndex :type Integer) (bFromSweep :type Boolean) (SweepResult :type "HitResult Structure (by ref)"))
  (bind _extractionui (`self.ExtractionUI`))
  (if (`self.CanExecute` OtherActor)
    (`|ExecutionSequence`
      (:`then_0`
        (`Widget.SetVisibility` _extractionui "Visible")
        (`UserWidget.PlayAnimation` _extractionui (`/Game/ProjectGrizzly/Map/ExtractionPoint/ExtractionWidget.FadeIn` _extractionui) 0.0 1 "Forward" 1.0 false))
      (:`then_1`
        (`KismetSystemLibrary.K2_ClearAndInvalidateTimerHandle` (`self.FadeoutTimer`)))
      (:`then_2`
        (set `self.ExtractionTime` (`self.StartExtractionTime`))
        (bind _returnvalue (`KismetSystemLibrary.K2_SetTimerDelegate` (`|CreateDelegate` :!event `UpdateExtraction`) 0.1 true))
        (set `self.ExtractionTimer` _returnvalue)))))

(event `UpdateExtraction`
  (bind _output_get (set `self.ExtractionTime` (`KismetMathLibrary.FClamp` (- (`self.ExtractionTime`) 0.1) 0.0 (`self.StartExtractionTime`))))
  (if (`KismetMathLibrary.NearlyEqual_FloatFloat` _output_get)
    (bind _returnvalue (`|CreateWidget` "/Game/ProjectGrizzly/UI/FadeInOut.FadeInOut_C" (`GameplayStatics.GetPlayerController` 0)))
    (add `/Game/ProjectGrizzly/UI/FadeInOut.OnFadeOutFinished` _returnvalue (`|CreateDelegate` :!event `Disconnect`))
    (`UserWidget.AddToViewport` _returnvalue 0)
    (`UserWidget.PlayAnimation` _returnvalue (`/Game/ProjectGrizzly/UI/FadeInOut.FadeOut` _returnvalue) 0.0 1 "Forward" 0.5 false)))

(event `self.Cube.OnComponentEndOverlap`
  (params (OverlappedComponent :type "PrimitiveComponent Object Reference") (OtherActor :type "Actor Object Reference") (OtherComp :type "PrimitiveComponent Object Reference") (OtherBodyIndex :type Integer))
  (bind _extractionui (`self.ExtractionUI`))
  (if (`self.CanExecute` OtherActor)
    (`|ExecutionSequence`
      (:`then_0`
        (`KismetSystemLibrary.K2_ClearAndInvalidateTimerHandle` (`self.ExtractionTimer`)))
      (:`then_1`
        (bind _returnvalue (`KismetSystemLibrary.K2_SetTimerDelegate` (delegate `StopExtraction`) 0.5))
        (set `self.FadeoutTimer` _returnvalue))
      (:`then_2`
        (`UserWidget.PlayAnimation` _extractionui (`/Game/ProjectGrizzly/Map/ExtractionPoint/ExtractionWidget.FadeOut` _extractionui) 0.0 1 "Forward" 1.0 false)))))

(event `StopExtraction`
  (`Widget.SetVisibility` (`self.ExtractionUI`) "Collapsed"))

(fn `CanExecute`
  (params (Actor :type "Actor Object Reference"))
  (returns (Local :type Boolean))
  (bind _asbp_player (cast `/Game/ProjectGrizzly/Character/BP_Player` Actor)
    (:`then`
      (return (`Pawn.IsLocallyControlled` _asbp_player)))
    (:`CastFailed`
      (return false))))

(fn `Disconnect`
  (bind _asbp_grizzly_pc (cast `/Game/ProjectGrizzly/Character/BP_GrizzlyPC` (`GameplayStatics.GetPlayerController` 0)))
  (`/Game/ProjectGrizzly/Character/BP_GrizzlyPC.SaveInventory` _asbp_grizzly_pc)
  (`KismetSystemLibrary.ExecuteConsoleCommand` "disconnect" null))

(fn `UserConstructionScript`)