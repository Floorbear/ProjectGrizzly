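; Lobby player controller that shows the lobby UI and handles joining a server.
; On BeginPlay it creates BP_LobbyUI, switches input to UI only and shows the mouse cursor.
; JoinServer opens the Loading level, passing the server IP joined with the port through the MapName option instead of connecting directly.
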(event `self.ReceiveBeginPlay`
  (bind _returnvalue (`|CreateWidget` "/Game/ProjectGrizzly/Lobby/Lobby/BP_LobbyUI.BP_LobbyUI_C" self))
  (`UserWidget.AddToViewport` _returnvalue 0)
  (`WidgetBlueprintLibrary.SetInputMode_UIOnlyEx` self null)
  (set `self.bShowMouseCursor` true))

(event `JoinServer`
  (params (ServerIP :type String))
  (`GameplayStatics.OpenLevel` "Loading" true (`KismetStringLibrary.Concat_StrStr` "MapName=" (`KismetStringLibrary.Concat_StrStr` ServerIP (`self.Port`)))))

(fn `UserConstructionScript`)