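; Projectile bullet for ProjectGrizzly that delivers impact effects and damage through the Gameplay Ability System.
; On the authority, box hits trigger particles and a crack-sound RPC before delayed destruction, while overlaps with non-instigators trigger particles and damage living characters.
; Particles and damage use effect specs carrying the hit result, and the crack sound skips locally controlled player shooters.
; AI threat propagation on impact is present but disconnected.
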(event `self.ReceiveBeginPlay`)

(event `self.ReceiveTick`
  (params (DeltaSeconds :type "Float (single-precision)")))

(event `PlayCrackSound_RPC`
  (params (Instigator :type "Pawn Object Reference") (Location :type "Vector Structure"))
  (`/Engine/EditorBlueprintResources/StandardMacros.IsValid` (`AIBlueprintHelperLibrary.GetAIController` Instigator)
    (:`Is Valid`
      (`self.PlayCrackSound` Location))
    (:`Is Not Valid`
      (`/Engine/EditorBlueprintResources/StandardMacros.IsValid` Instigator
        (:`Is Valid`
          (if (not (`Pawn.IsLocallyControlled` Instigator))
            (`self.PlayCrackSound` Location)))
        (:`Is Not Valid`
          (`self.PlayCrackSound` Location))))))

(event `self.Box.OnComponentHit`
  (params (HitComponent :type "PrimitiveComponent Object Reference") (OtherActor :type "Actor Object Reference") (OtherComp :type "PrimitiveComponent Object Reference") (NormalImpulse :type "Vector Structure") (Hit :type "HitResult Structure (by ref)"))
  (bind _returnvalue (`self.GetInstigator`))
  (`/Engine/EditorBlueprintResources/StandardMacros.IsValid` _returnvalue
    (:`Is Valid`
      (if (`self.HasAuthority` _returnvalue)
        (bind _ascpp_playable_character (cast `CPP_PlayableCharacter` _returnvalue))
        (`self.CreateParticle` Hit_Location Hit_ImpactNormal)
        (`self.PlayCrackSound_RPC` (`self.GetInstigator`) Hit_Location)
        (`KismetSystemLibrary.Delay` 0.2)
        (`self.K2_DestroyActor`)
        (else
          (`self.K2_DestroyActor`))))
    (:`Is Not Valid`
      (`self.K2_DestroyActor`))))

(event `self.Box.OnComponentBeginOverlap`
  (params (OverlappedComponent :type "PrimitiveComponent Object Reference") (OtherActor :type "Actor Object Reference") (OtherComp :type "PrimitiveComponent Object Reference") (OtherBodyIndex :type Integer) (bFromSweep :type Boolean) (SweepResult :type "HitResult Structure (by ref)"))
  (bind _returnvalue (`self.GetInstigator`))
  (bind (_bblockinghit _binitialoverlap _time _distance _location _impactpoint _normal _impactnormal _physmat _hitactor _hitcomponent _hitbonename) (`GameplayStatics.BreakHitResult` SweepResult))
  (if (`self.HasAuthority` _returnvalue)
    (if (!= _returnvalue _hitactor)
      (`/Engine/EditorBlueprintResources/ActorMacros.Switch Has Authority`
        (:`Authority`
          (`self.CreateParticle` _location _impactnormal _hitactor)
          (`self.ApplyDamageEffect` _hitactor SweepResult)
          (`self.K2_DestroyActor`))))))

(fn `ApplyDamageEffect`
  (params (HitActor :type "Actor Object Reference") (HitResult :type "HitResult Structure"))
  (bind _damageeffecthandle (`self.DamageEffectHandle`))
  (bind _ascpp_pgcharacter (cast `CPP_PGCharacter` HitActor))
  (if (not (`CPP_PGCharacter.IsDead` _ascpp_pgcharacter))
    (bind _ascpp_pgcharacter_2 (cast `CPP_PGCharacter` (`self.GetInstigator`)))
    (bind _returnvalue (`AbilitySystemBlueprintLibrary.GetEffectContext` _damageeffecthandle))
    (`AbilitySystemBlueprintLibrary.EffectContextAddHitResult` _returnvalue HitResult)
    (`AbilitySystemComponent.BP_ApplyGameplayEffectSpecToTarget` (`AbilitySystemBlueprintLibrary.GetAbilitySystemComponent` _ascpp_pgcharacter_2) _damageeffecthandle (`AbilitySystemBlueprintLibrary.GetAbilitySystemComponent` _ascpp_pgcharacter))))

(fn `CreateParticle`
  (params (HitLocation :type "Vector Structure") (HitNormal :type "Vector Structure") (HitActor :type "Actor Object Reference"))
  (bind _hitparticleeffecthandle (`self.HitParticleEffectHandle`))
  (bind _ascpp_pgcharacter (cast `CPP_PGCharacter` (`self.GetInstigator`)))
  (bind _returnvalue (`AbilitySystemBlueprintLibrary.GetEffectContext` _hitparticleeffecthandle))
  (if (`AbilitySystemBlueprintLibrary.EffectContextIsValid` _returnvalue)
    (`AbilitySystemBlueprintLibrary.EffectContextAddHitResult` _returnvalue (`GameplayStatics.MakeHitResult` false false 0.0 0.0 HitLocation (0.0 0.0 0.0) HitNormal (0.0 0.0 1.0) null HitActor))
    (`AbilitySystemComponent.BP_ApplyGameplayEffectSpecToSelf` (`AbilitySystemBlueprintLibrary.GetAbilitySystemComponent` _ascpp_pgcharacter) _hitparticleeffecthandle)))

(fn `OverlapThreat`
  (params (SpawnLocation :type "Vector Structure") (ThreatRadius :type "Float (double-precision)"))
  (returns (ThreatendActors :type "Array of Actor Object Reference"))
  (locals (NewLocalVar_0 :type "Array of Actor Object Reference"))
  (bind _outactors (`KismetSystemLibrary.SphereOverlapActors` SpawnLocation ThreatRadius (`|MakeArray` (enumliteral `EObjectTypeQuery` "ObjectTypeQuery3")) "/Script/ProjectGrizzly.CPP_PGCharacter" (`|MakeArray` (`self.GetInstigator`) :!type "Actor Object Reference")))
  (return _outactors))

(fn `PlayCrackSound`
  (params (Location :type "Vector Structure"))
  (locals (NewLocalVar_1 :type "Array of SoundBase Object Reference"))
  (`GameplayStatics.PlaySoundAtLocation` (`KismetArrayLibrary.Array_Random` (`local.NewLocalVar_1`)) Location (struct) 1.0 1.0 0.0 null null null null))

(fn `UserConstructionScript`)