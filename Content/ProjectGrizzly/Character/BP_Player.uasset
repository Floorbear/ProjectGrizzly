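; Player character Blueprint for Project Grizzly, handling movement, mouse look and debug hotkeys on top of inherited character functions.
; Mouse look nudges the first-person hands mesh for sway, while locally controlled Tick updates interaction, high-ready interpolation and hand return.
; Keys respawn the dead player through BP_GrizzlyPC, spawn an armed Bandit AI and use a medkit.
; BPHandSway (clamped rotational sway) and BPSpawnStalker are helpers not called here.
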(event `InputAxis|Move Right / Left`
  (params (AxisValue :type "Float (single-precision)"))
  ;[1 1 1] Movement
  (if (not (`self.IsDead`))
    (`self.AddMovementInput` (`self.GetActorRightVector`) AxisValue)
    (`self.SetMoveRightAxis` AxisValue)))

(event `self.ReceiveBeginPlay`
  (`self.SetCharacterModel` "Merc_2a"))

(event `InputAxis|Move Forward / Backward`
  (params (AxisValue :type "Float (single-precision)"))
  ;[1 1 1] Movement
  (if (not (`self.IsDead`))
    (`self.AddMovementInput` (`self.GetActorForwardVector`) AxisValue)
    (`self.SetMoveForwardAxis` AxisValue)))

(event `InputAxis|Look Up / Down Mouse`
  (params (AxisValue :type "Float (single-precision)"))
  ;[1 1 1] Movement
  (if (not (`self.IsDead`))
    (`self.AddControllerPitchInput` AxisValue)
    ;;[1 1 1] HandSway
    (bind _output_get (set `self.MouseYDelta` AxisValue))
    (bind _returnvalue (`self.GetHandsMeshComponent`))
    (`SceneComponent.K2_AddRelativeLocation` _returnvalue (`KismetMathLibrary.MakeVector` 0.0 0.0 (* _output_get 0.1)) false false)))

(event `self.ReceiveTick`
  (params (DeltaSeconds :type "Float (single-precision)"))
  (if (and (`self.IsLocallyControlled`) (!= (`AbilitySystemBlueprintLibrary.GetAbilitySystemComponent` self) null))
    (`self.UpdateFrontInteraction` DeltaSeconds)
    (`self.UpdateHighReadyInterpo` DeltaSeconds)
    (`self.ReturnToHands` DeltaSeconds)))

(event `InputAxis|Turn Right / Left Mouse`
  (params (AxisValue :type "Float (single-precision)"))
  ;[1 1 1] Movement
  (if (not (`self.IsDead`))
    (`self.AddControllerYawInput` AxisValue)
    ;;[1 1 1] HandSway
    (bind _output_get (set `self.MouseXDelta` AxisValue))
    (bind _returnvalue (`self.GetHandsMeshComponent`))
    (`SceneComponent.K2_AddRelativeLocation` _returnvalue (`KismetMathLibrary.MakeVector` 0.0 (* _output_get -0.06)) false false)))

(event `Key|K`
  (params (Key :type "Key Structure"))
  (:`Pressed`
    (if (`self.IsDead`)
      (bind _returnvalue (`self.IsMyComputer`))
      (if _returnvalue
        (bind _asbp_grizzly_pc (cast `/Game/ProjectGrizzly/Character/BP_GrizzlyPC` (`self.GetController`)))
        (`/Game/ProjectGrizzly/Character/BP_GrizzlyPC.RespawnActor` _asbp_grizzly_pc)
        (`GrizzlyPC.OffDeadNotificationUI` _asbp_grizzly_pc)))))

(event `Key|J`
  (params (Key :type "Key Structure"))
  (:`Pressed`
    (`self.SpawnMerc`)))

(event `Key|H`
  (params (Key :type "Key Structure"))
  ;[1 1 1] Debug
)

(event `SpawnMerc`
  (bind _outactors (`GameplayStatics.GetAllActorsOfClass` "/Script/Engine.PlayerStart"))
  ;[1 1 1] Debug
  (`CPP_AIPlayableCharacter.SpawnAIPlayableCharacter` "/Game/ProjectGrizzly/Character/BP_AIPlayableCharacter.BP_AIPlayableCharacter_C" (make `AIPlayableCharacterSpawnParameter` "Bandit" "Bandit_3a" "Weapon_AKM") "/Game/ProjectGrizzly/Character/AI/BehaviorTrees/BT_AIMain.BT_AIMain" (`self.K2_GetActorLocation` (`|GetArrayItem` _outactors)) (struct) false null))

(event `SpawnBandit`
  ;[1 1 1] Debug
  (bind _outactors (`GameplayStatics.GetAllActorsOfClass` "/Script/Engine.PlayerStart"))
  (bind _output (`|GetArrayItem` _outactors 1))
  (`self.BP_SpawnStalker` "Bandit" "Bandit_3a" (`self.K2_GetActorLocation` _output) (`self.K2_GetActorRotation` _output)))

(event `Key|Five`
  (params (Key :type "Key Structure"))
  (:`Pressed`
    (bind _returnvalue (`InventoryComponent.FindItemFromInventory` (`self.InventoryComponent`) "Medical_Medickit"))
    (`self.TryUseItem` _returnvalue)))

(fn `BP_HandSway`
  (params (BP_DeltaTime :type "Float (double-precision)"))
  (locals (BP_FinalHandSway :type "Rotator Structure") (BP_InitHandSway :type "Rotator Structure" :default (struct :`Yaw` -90.0)))
  (bind (_bp_inithandsway_roll _bp_inithandsway_pitch _bp_inithandsway_yaw) (`KismetMathLibrary.BreakRotator` (`local.BP_InitHandSway`)))
  (bind (_bp_inithandsway_roll_2 _bp_inithandsway_pitch_2 _bp_inithandsway_yaw_2) (`KismetMathLibrary.BreakRotator` (`local.BP_InitHandSway`)))
  (bind _bp_maxswaydegree (`self.BP_MaxSwayDegree`))
  (bind (_bp_finalhandsway_roll _bp_finalhandsway_pitch _bp_finalhandsway_yaw) (`KismetMathLibrary.BreakRotator` (`local.BP_FinalHandSway`)))
  (bind (_bp_inithandsway_roll_3 _bp_inithandsway_pitch_3 _bp_inithandsway_yaw_3) (`KismetMathLibrary.BreakRotator` (`local.BP_InitHandSway`)))
  (bind _returnvalue (`KismetMathLibrary.Abs` (`self.BP_MaxSwayDegree`)))
  (bind _returnvalue_2 (* _returnvalue -1.0))
  (bind _returnvalue_3 (* (`KismetMathLibrary.FClamp` (+ (`self.MouseXDelta`) (`self.BP_HandSwayHori`)) -1.0) _bp_maxswaydegree))
  ;[1 1 1] Pitch : Roll 값임
  (set `local.BP_FinalHandSway` (`KismetMathLibrary.MakeRotator` (* _bp_maxswaydegree (`self.MouseYDelta`)) _returnvalue_3 _returnvalue_3))
  (bind _returnvalue_4 (`self.GetHandsMeshComponent`))
  (`SceneComponent.K2_SetRelativeRotation` _returnvalue_4 (`KismetMathLibrary.MakeRotator` (`KismetMathLibrary.FClamp` (.roll (`KismetMathLibrary.RInterpTo` (`SceneComponent.RelativeRotation` _returnvalue_4) (`KismetMathLibrary.MakeRotator` (+ _bp_inithandsway_roll_3 _bp_finalhandsway_roll) (- _bp_inithandsway_pitch_3 _bp_finalhandsway_pitch) (+ _bp_inithandsway_yaw_3 _bp_finalhandsway_yaw)) BP_DeltaTime 4.0)) _returnvalue_2 _returnvalue) (`KismetMathLibrary.FClamp` (.pitch (`KismetMathLibrary.RInterpTo` (`SceneComponent.RelativeRotation` _returnvalue_4) (`KismetMathLibrary.MakeRotator` (+ _bp_inithandsway_roll_3 _bp_finalhandsway_roll) (- _bp_inithandsway_pitch_3 _bp_finalhandsway_pitch) (+ _bp_inithandsway_yaw_3 _bp_finalhandsway_yaw)) BP_DeltaTime 4.0)) _returnvalue_2 _returnvalue) (`KismetMathLibrary.FClamp` (.yaw (`KismetMathLibrary.RInterpTo` (`SceneComponent.RelativeRotation` _returnvalue_4) (`KismetMathLibrary.MakeRotator` (+ _bp_inithandsway_roll_3 _bp_finalhandsway_roll) (- _bp_inithandsway_pitch_3 _bp_finalhandsway_pitch) (+ _bp_inithandsway_yaw_3 _bp_finalhandsway_yaw)) BP_DeltaTime 4.0)) (+ (* (`KismetMathLibrary.Abs` (`self.BP_MaxSwayDegree`)) -1.0) _bp_inithandsway_yaw) (+ (`KismetMathLibrary.Abs` (`self.BP_MaxSwayDegree`)) _bp_inithandsway_yaw_2))) false false))

(fn `BP_SpawnStalker`
  (params (Faction :type "EFaction Enum" :default "NonSet") (Model :type "ECharacterModel Enum" :default "Merc_2a") (Location :type "Vector Structure") (Rotation :type "Rotator Structure"))
  (bind _returnvalue (`AIBlueprintHelperLibrary.SpawnAIFromClass` "/Game/ProjectGrizzly/Character/BP_AIPlayableCharacter.BP_AIPlayableCharacter_C" null Location Rotation false null))
  (bind _asbp_aiplayable_character (cast `/Game/ProjectGrizzly/Character/BP_AIPlayableCharacter` _returnvalue))
  (`FactionComponent.SetFaction` (`self.GetFactionComponent` _asbp_aiplayable_character) Faction)
  (`self.SetCharacterModel` _asbp_aiplayable_character Model))

(fn `UserConstructionScript`)