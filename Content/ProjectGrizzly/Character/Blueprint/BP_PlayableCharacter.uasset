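; Playable character Blueprint that handles basic player movement and mouse look through input axis events.
; Move axes feed CharacterMovement.AddInputVector directly, using the actor's forward vector for forward/back and the control rotation's right vector for strafing.
; Mouse axes drive controller yaw and pitch input.
; BeginPlay, Tick, overlap and the construction script are empty.
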(event `InputAxis|Move Forward / Backward`
  (params (AxisValue :type "Float (single-precision)"))
  (`PawnMovementComponent.AddInputVector` (`self.CharacterMovement`) (* AxisValue (`self.GetActorForwardVector`)) false))

(event `InputAxis|Move Right / Left`
  (params (AxisValue :type "Float (single-precision)"))
  (`PawnMovementComponent.AddInputVector` (`self.CharacterMovement`) (* AxisValue (`KismetMathLibrary.GetRightVector` (`self.GetControlRotation`))) false))

(event `InputAxis|Look Up / Down Mouse`
  (params (AxisValue :type "Float (single-precision)"))
  (`self.AddControllerPitchInput` AxisValue))

(event `InputAxis|Turn Right / Left Mouse`
  (params (AxisValue :type "Float (single-precision)"))
  (`self.AddControllerYawInput` AxisValue))

(fn `UserConstructionScript`)