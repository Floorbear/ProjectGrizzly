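; Player controller for Project Grizzly that builds the local UI (HUD, inventory, death notice) and handles respawning.
; BeginPlay branches on game phase: Loadout loads the player inventory and opens it against the game mode's stash, while Playing only creates the UI for the local controller.
; Inventory saves to and loads from the GameInstance under a "Player" key.
; Numpad keys grant test weapons, ammo and items.
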(event `self.ReceiveBeginPlay`
  (switch `EGamePhase` (`self.GetGamePhase`)
    (:`Loadout`
      (`self.ShowOnLoadoutLevel`))
    (:`Playing`
      (if (`self.IsLocalController`)
        (`self.CreateUI`)))))

(event `SpawnClientHUD`
  (`self.BP Spawn Client HUD`))

(event `self.OnDeadNotificationUI`
  (`UserWidget.AddToViewport` (`self.DeadNotificationUI`) 0)
  (`Widget.RemoveFromParent` (`self.InventoryUI`)))

(event `self.OffDeadNotificationUI`
  (`Widget.RemoveFromParent` (`self.DeadNotificationUI`)))

(event `RespawnActor`
  (bind _asbp_grizzly_game_mode (cast `/Game/ProjectGrizzly/BP_GrizzlyGameMode` (`GameplayStatics.GetGameMode`)))
  (`/Game/ProjectGrizzly/BP_GrizzlyGameMode.SpawnGrizzlyActor` _asbp_grizzly_game_mode self)
  (`self.Respawn_Client`))

(event `Key|NumPadFour`
  (params (Key :type "Key Structure"))
  (:`Pressed`
    (`InventoryComponent.AddItemToInventory` (`self.GetInventoryComponent`) "Weapon_Colt" 1)))

(event `Respawn_Client`
  (`self.CreateInventoryUI`))

(event `Key|NumPadFive`
  (params (Key :type "Key Structure"))
  (:`Pressed`
    (`InventoryComponent.AddItemToInventory` (`self.GetInventoryComponent`) "Weapon_AKM" 1)))

(event `InputAction|Inventory`
  (params (Key :type "Key Structure"))
  (:`Pressed`
    (`self.BP_Show Inventory` (struct))))

(event `Key|NumPadSix`
  (params (Key :type "Key Structure"))
  (:`Pressed`
    (`InventoryComponent.AddItemToInventory` (`self.GetInventoryComponent`) "Ammo_7.62x39mm" 10)))

(event `self.ShowInventory`
  (params (_Parameter :type "InventoryUI_Parameter Structure"))
  (if (`self.IsLocalPlayerController` self)
    (`self.BP_Show Inventory` _Parameter)))

(event `Key|NumPadThree`
  (params (Key :type "Key Structure"))
  (:`Pressed`
    (`InventoryComponent.AddItemToInventory` (`self.GetInventoryComponent`) "Etc_LonerPatch" 1)))

(fn `BP Spawn Client HUD`
  (if (`|EnumEquality` (`self.GetGamePhase`) "Playing")
    (bind _asbp_grizzly_ps (cast `/Game/ProjectGrizzly/Character/BP_GrizzlyPS` (`self.PlayerState`))
      (:`then`
        _)
      (:`CastFailed`
        _))
    (bind _returnvalue (`|CreateWidget` "/Game/ProjectGrizzly/UI/ClientHUD.ClientHUD_C" self self _asbp_grizzly_ps))
    (`UserWidget.AddToViewport` _returnvalue 0)))

(fn `BP_LoadPlayerInventory`
  (bind _asgrizzly_game_instance (cast `GrizzlyGameInstance` (`GameplayStatics.GetGameInstance`)))
  (bind _returnvalue (`GrizzlyGameInstance.GetInventoryFromKey` _asgrizzly_game_instance "Player"))
  (`InventoryComponent.SetInventory` (`self.GetInventoryComponent`) _returnvalue))

(fn `BP_Show Inventory`
  (params (InventoryUI_Parameter :type "InventoryUI_Parameter Structure"))
  (bind _bp_inventoryui (`self.BP_InventoryUI`))
  (`|ExecutionSequence`
    (:`then_0`
      (`Widget.SetFocus` _bp_inventoryui)
      (`Widget.SetVisibility` _bp_inventoryui "SelfHitTestInvisible")
      (`WidgetBlueprintLibrary.SetInputMode_UIOnlyEx` self _bp_inventoryui "LockInFullscreen"))
    (:`then_1`
      (switch `EInventoryCategory` (`.InventoryCategory` (break `InventoryUI_Parameter` InventoryUI_Parameter))
        (:`ItemContainer`
          (`/Game/ProjectGrizzly/Item/BP_InventoryUI.SetOpponentInventory` (`self.BP_InventoryUI`) (`local.InventoryUI_Parameter`)))))))

(fn `CreateInventoryUI`
  (bind _returnvalue (`|CreateWidget` "/Game/ProjectGrizzly/Item/BP_InventoryUI.BP_InventoryUI_C" self))
  (bind _output_get (set `self.BP_InventoryUI` _returnvalue))
  (set `self.InventoryUI` _output_get)
  (`UserWidget.AddToViewport` _returnvalue 0)
  (`/Game/ProjectGrizzly/Item/BP_InventoryUI.Init` _output_get 10))

(fn `CreateUI`
  (`self.SpawnClientHUD`)
  (bind _returnvalue (`|CreateWidget` "/Game/ProjectGrizzly/UI/DeadNotification.DeadNotification_C" self))
  (set `self.DeadNotificationUI` _returnvalue)
  (`WidgetBlueprintLibrary.SetInputMode_GameOnly` self)
  (`self.CreateInventoryUI`))

(fn `SaveInventory`
  (bind _asgrizzly_game_instance (cast `GrizzlyGameInstance` (`GameplayStatics.GetGameInstance`)))
  (`GrizzlyGameInstance.SetInventory` _asgrizzly_game_instance (`InventoryComponent.ToInventoryData` (`self.GetInventoryComponent`) "Player")))

(fn `ShowOnLoadoutLevel`
  (locals (GM_Loadout :type "/Game/ProjectGrizzly/Lobby/Title/Loadout/GM_Loadout Object Reference"))
  (bind _asgm_loadout (cast `/Game/ProjectGrizzly/Lobby/Title/Loadout/GM_Loadout` (`GameplayStatics.GetGameMode`)))
  (set `local.GM_Loadout` _asgm_loadout)
  (`|ExecutionSequence`
    (:`then_0`
      (`self.CreateUI`))
    (:`then_1`
      (`self.BP_LoadPlayerInventory`))
    (:`then_2`
      (`self.ShowInventory` (make `InventoryUI_Parameter` "ItemContainer" (`CPP_Crate.Inventory` (`/Game/ProjectGrizzly/Lobby/Title/Loadout/GM_Loadout.Stash` (`local.GM_Loadout`))))))))

(fn `UserConstructionScript`)