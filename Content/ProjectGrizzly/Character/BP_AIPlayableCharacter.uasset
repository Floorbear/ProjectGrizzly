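; Playable character Blueprint that adds mouse-driven sway to its hands mesh.
; Construction Script caches the camera's relative location; nothing here reads it back.
; HandSway scales mouse deltas by a max sway angle, offsets the initial hand rotation and interpolates toward it using the passed delta time.
; Each axis is clamped to the sway limit, with only yaw's range centered on its initial value.
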(fn `HandSway`
  (params (BP_DeltaTime :type "Float (double-precision)"))
  (locals (BP_FinalHandSway :type "Rotator Structure") (BP_InitHandSway :type "Rotator Structure" :default (struct :`Yaw` -90.0)))
  (bind (_bp_inithandsway_roll _bp_inithandsway_pitch _bp_inithandsway_yaw) (`KismetMathLibrary.BreakRotator` (`local.BP_InitHandSway`)))
  (bind (_bp_inithandsway_roll_2 _bp_inithandsway_pitch_2 _bp_inithandsway_yaw_2) (`KismetMathLibrary.BreakRotator` (`local.BP_InitHandSway`)))
  (bind _bp_maxswaydegree (`self.BP_MaxSwayDegree`))
  (bind (_bp_finalhandsway_roll _bp_finalhandsway_pitch _bp_finalhandsway_yaw) (`KismetMathLibrary.BreakRotator` (`local.BP_FinalHandSway`)))
  (bind (_bp_inithandsway_roll_3 _bp_inithandsway_pitch_3 _bp_inithandsway_yaw_3) (`KismetMathLibrary.BreakRotator` (`local.BP_InitHandSway`)))
  (bind _returnvalue (`KismetMathLibrary.Abs` (`self.BP_MaxSwayDegree`)))
  (bind _returnvalue_2 (* (`self.MouseXDelta`) _bp_maxswaydegree))
  (bind _returnvalue_3 (* _returnvalue -1.0))
  ;[1 1 1] Pitch : Roll 값임
  (set `local.BP_FinalHandSway` (`KismetMathLibrary.MakeRotator` (* _bp_maxswaydegree (`self.MouseYDelta`)) _returnvalue_2 _returnvalue_2))
  (bind _returnvalue_4 (`self.GetHandsMeshComponent`))
  (`SceneComponent.K2_SetRelativeRotation` _returnvalue_4 (`KismetMathLibrary.MakeRotator` (`KismetMathLibrary.FClamp` (.roll (`KismetMathLibrary.RInterpTo` (`SceneComponent.RelativeRotation` _returnvalue_4) (`KismetMathLibrary.MakeRotator` (+ _bp_inithandsway_roll_3 _bp_finalhandsway_roll) (- _bp_inithandsway_pitch_3 _bp_finalhandsway_pitch) (+ _bp_inithandsway_yaw_3 _bp_finalhandsway_yaw)) BP_DeltaTime 4.0)) _returnvalue_3 _returnvalue) (`KismetMathLibrary.FClamp` (.pitch (`KismetMathLibrary.RInterpTo` (`SceneComponent.RelativeRotation` _returnvalue_4) (`KismetMathLibrary.MakeRotator` (+ _bp_inithandsway_roll_3 _bp_finalhandsway_roll) (- _bp_inithandsway_pitch_3 _bp_finalhandsway_pitch) (+ _bp_inithandsway_yaw_3 _bp_finalhandsway_yaw)) BP_DeltaTime 4.0)) _returnvalue_3 _returnvalue) (`KismetMathLibrary.FClamp` (.yaw (`KismetMathLibrary.RInterpTo` (`SceneComponent.RelativeRotation` _returnvalue_4) (`KismetMathLibrary.MakeRotator` (+ _bp_inithandsway_roll_3 _bp_finalhandsway_roll) (- _bp_inithandsway_pitch_3 _bp_finalhandsway_pitch) (+ _bp_inithandsway_yaw_3 _bp_finalhandsway_yaw)) BP_DeltaTime 4.0)) (+ (* (`KismetMathLibrary.Abs` (`self.BP_MaxSwayDegree`)) -1.0) _bp_inithandsway_yaw) (+ (`KismetMathLibrary.Abs` (`self.BP_MaxSwayDegree`)) _bp_inithandsway_yaw_2))) false false))

(fn `UserConstructionScript`
  (set `self.BP_CameraLocation` (`SceneComponent.RelativeLocation` (`self.Camera`))))