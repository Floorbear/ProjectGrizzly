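; GA_Jump is a Gameplay Ability that makes the playable character jump.
; Activation is allowed only when the avatar casts to CPP_PlayableCharacter and its CanJump check passes.
; On activation it commits the ability, calls the character's Jump if the commit succeeds, and ends immediately in either case.
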(event `self.K2_ActivateAbility`
  (bind _returnvalue (`self.K2_CommitAbility`))
  (if _returnvalue
    (`Character.Jump` (`self.GetCharacter`))
    (`self.K2_EndAbility`)
    (else
      (`self.K2_EndAbility`))))

(fn `K2_CanActivateAbility`
  (params (ActorInfo :type "GameplayAbilityActorInfo Structure") (Handle :type "GameplayAbilitySpecHandle Structure"))
  (returns (RelevantTags :type "GameplayTagContainer Structure") (ReturnValue :type Boolean))
  (bind _ascpp_playable_character (cast `CPP_PlayableCharacter` (`.AvatarActor` (break `GameplayAbilityActorInfo` ActorInfo))))
  (return (struct) (`Character.CanJump` _ascpp_playable_character)))