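; Playable first-person character Blueprint handling movement, mouse look, aim-down-sights and AKM animations.
; Tick interpolates the hands mesh between its cached idle location and a zero offset while right mouse is held.
; HandSway turns mouse deltas into interpolated, clamped hand rotation.
; Left mouse plays hands and weapon fire montages, T plays a body-mesh reload montage, and first-person reload chains are unconnected.
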(event `InputAxis|Move Right / Left`
  (params (AxisValue :type "Float (single-precision)"))
  ;[1 1 1] Movement
  (`self.AddMovementInput` (`self.GetActorRightVector`) AxisValue)
  (set `self.MoveRightAxis` AxisValue))

(event `self.ReceiveBeginPlay`
  (bind _returnvalue (`self.GetHandsMeshComponent`))
  (set `self.BP_IdleHandLocation` (`SceneComponent.RelativeLocation` _returnvalue)))

(event `InputAxis|Move Forward / Backward`
  (params (AxisValue :type "Float (single-precision)"))
  ;[1 1 1] Movement
  (`self.AddMovementInput` (`self.GetActorForwardVector`) AxisValue)
  (set `self.MoveForwardAxis` AxisValue))

(event `InputAxis|Look Up / Down Mouse`
  (params (AxisValue :type "Float (single-precision)"))
  ;[1 1 1] Movement
  (`self.AddControllerPitchInput` AxisValue)
  (set `self.MouseYDelta` AxisValue))

(event `self.ReceiveTick`
  (params (DeltaSeconds :type "Float (single-precision)"))
  (`self.HandSway` DeltaSeconds)
  (if (`self.BP_bADS`)
    (bind _returnvalue (`self.GetHandsMeshComponent`))
    (`SceneComponent.K2_SetRelativeLocation` _returnvalue (`KismetMathLibrary.VInterpTo` (`SceneComponent.RelativeLocation` _returnvalue) (0.0 0.0 0.0) (`GameplayStatics.GetWorldDeltaSeconds`) 6.0) false false)
    (else
      (bind _returnvalue_2 (`self.GetHandsMeshComponent`))
      (`SceneComponent.K2_SetRelativeLocation` _returnvalue_2 (`KismetMathLibrary.VInterpTo` (`SceneComponent.RelativeLocation` _returnvalue_2) (`self.BP_IdleHandLocation`) (`GameplayStatics.GetWorldDeltaSeconds`) 6.0) false false))))

(event `InputAxis|Turn Right / Left Mouse`
  (params (AxisValue :type "Float (single-precision)"))
  ;[1 1 1] Movement
  (`self.AddControllerYawInput` AxisValue)
  (set `self.MouseXDelta` AxisValue))

(event `Key|RightMouseButton`
  (params (Key :type "Key Structure"))
  (:`Pressed`
    (set `self.BP_bADS` true))
  (:`Released`
    (set `self.BP_bADS` false)))

(event `Key|T`
  (params (Key :type "Key Structure"))
  (:`Pressed`
    (`AnimInstance.Montage_Play` (`SkeletalMeshComponent.GetAnimInstance` (`self.Mesh`)) "/Game/ProjectGrizzly/Character/Model/Animations/Montage_Torso2_Reload.Montage_Torso2_Reload" 1.0 "MontageLength" 0.0 true)))

(event `Key|R`
  (params (Key :type "Key Structure")))

(event `Key|LeftMouseButton`
  (params (Key :type "Key Structure"))
  (:`Pressed`
    (bind _returnvalue (`self.GetHandsMeshComponent`))
    (`|PlayMontage` _returnvalue "/Game/ProjectGrizzly/Character/FirstPersonHand/Animation/Akm/Montage_Hands_AKM_Shoot.Montage_Hands_AKM_Shoot"
      (:`then`
        (bind _returnvalue_2 (`self.GetFPWeaponMeshComponent`))
        (`|PlayMontage` _returnvalue_2 "/Game/ProjectGrizzly/Gun/Akm/Animations/Montage_AKM_Shoot.Montage_AKM_Shoot")))))

(fn `HandSway`
  (params (BP_DeltaTime :type "Float (double-precision)"))
  (locals (BP_FinalHandSway :type "Rotator Structure") (BP_InitHandSway :type "Rotator Structure" :default (struct :`Yaw` -90.0)))
  (bind (_bp_inithandsway_roll _bp_inithandsway_pitch _bp_inithandsway_yaw) (`KismetMathLibrary.BreakRotator` (`local.BP_InitHandSway`)))
  (bind (_bp_inithandsway_roll_2 _bp_inithandsway_pitch_2 _bp_inithandsway_yaw_2) (`KismetMathLibrary.BreakRotator` (`local.BP_InitHandSway`)))
  (bind _bp_maxswaydegree (`self.BP_MaxSwayDegree`))
  (bind (_bp_finalhandsway_roll _bp_finalhandsway_pitch _bp_finalhandsway_yaw) (`KismetMathLibrary.BreakRotator` (`local.BP_FinalHandSway`)))
  (bind (_bp_inithandsway_roll_3 _bp_inithandsway_pitch_3 _bp_inithandsway_yaw_3) (`KismetMathLibrary.BreakRotator` (`local.BP_InitHandSway`)))
  (bind _returnvalue (`KismetMathLibrary.Abs` (`self.BP_MaxSwayDegree`)))
  (bind _returnvalue_2 (* (`self.MouseXDelta`) _bp_maxswaydegree))
  (bind _returnvalue_3 (* _returnvalue -1.0))
  ;[1 1 1] Pitch : Roll 값임
  (set `local.BP_FinalHandSway` (`KismetMathLibrary.MakeRotator` (* _bp_maxswaydegree (`self.MouseYDelta`)) _returnvalue_2 _returnvalue_2))
  (bind _returnvalue_4 (`self.GetHandsMeshComponent`))
  (`SceneComponent.K2_SetRelativeRotation` _returnvalue_4 (`KismetMathLibrary.MakeRotator` (`KismetMathLibrary.FClamp` (.roll (`KismetMathLibrary.RInterpTo` (`SceneComponent.RelativeRotation` _returnvalue_4) (`KismetMathLibrary.MakeRotator` (+ _bp_inithandsway_roll_3 _bp_finalhandsway_roll) (- _bp_inithandsway_pitch_3 _bp_finalhandsway_pitch) (+ _bp_inithandsway_yaw_3 _bp_finalhandsway_yaw)) BP_DeltaTime 4.0)) _returnvalue_3 _returnvalue) (`KismetMathLibrary.FClamp` (.pitch (`KismetMathLibrary.RInterpTo` (`SceneComponent.RelativeRotation` _returnvalue_4) (`KismetMathLibrary.MakeRotator` (+ _bp_inithandsway_roll_3 _bp_finalhandsway_roll) (- _bp_inithandsway_pitch_3 _bp_finalhandsway_pitch) (+ _bp_inithandsway_yaw_3 _bp_finalhandsway_yaw)) BP_DeltaTime 4.0)) _returnvalue_3 _returnvalue) (`KismetMathLibrary.FClamp` (.yaw (`KismetMathLibrary.RInterpTo` (`SceneComponent.RelativeRotation` _returnvalue_4) (`KismetMathLibrary.MakeRotator` (+ _bp_inithandsway_roll_3 _bp_finalhandsway_roll) (- _bp_inithandsway_pitch_3 _bp_finalhandsway_pitch) (+ _bp_inithandsway_yaw_3 _bp_finalhandsway_yaw)) BP_DeltaTime 4.0)) (+ (* (`KismetMathLibrary.Abs` (`self.BP_MaxSwayDegree`)) -1.0) _bp_inithandsway_yaw) (+ (`KismetMathLibrary.Abs` (`self.BP_MaxSwayDegree`)) _bp_inithandsway_yaw_2))) false false))

(fn `UserConstructionScript`)